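; Player Blueprint that handles Enhanced Input movement on the XY plane and toggles the pause menu.
; Movement offsets the actor by a fixed step from Sweep, which sphere-traces X and Y separately, ignoring BP_Shape actors found at BeginPlay.
; Blocked axes are zeroed and the remainder normalized, so the player slides along walls at full speed.
; Pausing creates WBP_PauseMenu and switches input mode; the Unpause event shares the resume path.
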(event Custom|Unpause
  (bind _returnvalue (Game|GetPlayerController 0))
  ;[0 0 0] Pause
  (Widget|RemovefromParent (stale Input|EnhancedActionEvents|EnhancedInputActionIA_Pause _returnvalue_3))
  (Input|SetInputModeGameOnly _returnvalue false)
  (Variables|/Script/Engine.PlayerController|SetbShowMouseCursor _returnvalue false)
  (Game|SetGamePaused false))

(event Input|EnhancedActionEvents|EnhancedInputActionIA_Pause
  (params (ActionValue :type Boolean) (ElapsedSeconds :type Float%20%28double-precision%29) (TriggeredSeconds :type Float%20%28double-precision%29) (InputAction :type Input%20Action%20Object%20Reference :default "/Game/Input/IA_Pause.IA_Pause"))
  (bind _returnvalue (Game|GetPlayerController 0))
  (bind _returnvalue_2 (Game|GetPlayerController 0))
  ;[0 0 0] Pause
  (:Started
    (if (Game|IsGamePaused)
      (Widget|RemovefromParent (stale _returnvalue_3))
      (Input|SetInputModeGameOnly _returnvalue false)
      (Variables|/Script/Engine.PlayerController|SetbShowMouseCursor _returnvalue false)
      (Game|SetGamePaused false)
      (else
        (bind _returnvalue_3 (Game|ConstructObjectfromClass "/Game/UI/WBP_PauseMenu.WBP_PauseMenu_C"))
        (UserInterface|Viewport|AddtoViewport _returnvalue_3 0)
        (Input|SetInputModeGameandUI _returnvalue_2 0 "DoNotLock" true false)
        (Variables|/Script/Engine.PlayerController|SetbShowMouseCursor _returnvalue_2 true)
        (Game|SetGamePaused true)))))

(event Input|EnhancedActionEvents|EnhancedInputActionIA_Move
  (params (ActionValue :type Vector%202D%20Structure) (ElapsedSeconds :type Float%20%28double-precision%29) (TriggeredSeconds :type Float%20%28double-precision%29) (InputAction :type Input%20Action%20Object%20Reference :default "/Game/Input/IA_Move.IA_Move"))
  (bind _returnvalue (Transformation|GetActorLocation))
  ;[0 0 0] Move Player
  (bind _new_velocity (CallFunction|Sweep _returnvalue ActionValue 25.0))
  (Transformation|SetActorLocation (+ _new_velocity _returnvalue) false false))

(event EventBeginPlay
  (bind _returnvalue (Game|GetPlayerController 0))
  (bind _returnvalue_2 (PlayerController|LocalPlayerSubsystems|GetEnhancedInputLocalPlayerSubsystem _returnvalue))
  ;[0 0 0] Begin Play
  (Utilities|IsValid _returnvalue_2
    (:Is%20Valid
      (Input|AddMappingContext _returnvalue_2 "/Game/Input/IMC_Default.IMC_Default" 0 "(bIgnoreAllPressedKeysUntilRelease=True,bForceImmediately=False,bNotifyUserSettings=False)")
      (bind _outactors (Actor|GetAllActorsOfClass "/Game/Actors/Shapes/BP_Shape.BP_Shape_C"))
      (Variables|Default|SetShapes%20To%20Ignore _outactors))))

(fn ConstructionScript)

(fn Sweep
  (params (Player%20Location :type Vector) (Action%20Value :type Vector%202D%20Structure) (Speed :type Float%20%28double-precision%29))
  (bind (_x _y) (Math|Vector2D|BreakVector2D Action%20Value))
  (LocalVariables|SetStart Player%20Location)
  (LocalVariables|SetVelocity%20Multiplier Speed)
  (LocalVariables|SetVelocity%20X _x)
  (LocalVariables|SetVelocity%20Y _y)
  (bind _returnvalue (Collision|SphereTraceByChannel (LocalVariables|GetStart) (Math|Vector|MakeVector (+ (* (LocalVariables|GetVelocity%20X) (LocalVariables|GetVelocity%20Multiplier)) (.X (Math|Vector|BreakVector (LocalVariables|GetStart)))) (.Y (Math|Vector|BreakVector (LocalVariables|GetStart))) (.Z (Math|Vector|BreakVector (LocalVariables|GetStart)))) 4e+01 "TraceTypeQuery1" false (Variables|Default|GetShapes%20To%20Ignore) "None" :!pinned true)) ; Sweep X axis
  (if _returnvalue ; If the player hits a wall
    (LocalVariables|SetVelocity%20X 0.0) ; Set his Velocity X to 0 so that he cant move in that direction
  )
  (bind _returnvalue_2 (Collision|SphereTraceByChannel (LocalVariables|GetStart) (Math|Vector|MakeVector (.X (Math|Vector|BreakVector (LocalVariables|GetStart))) (+ (.Y (Math|Vector|BreakVector (LocalVariables|GetStart))) (* (LocalVariables|GetVelocity%20Y) (LocalVariables|GetVelocity%20Multiplier))) (.Z (Math|Vector|BreakVector (LocalVariables|GetStart)))) 4e+01 "TraceTypeQuery1" false (Variables|Default|GetShapes%20To%20Ignore) "None" :!pinned true)) ; Sweep Y axis
  (if _returnvalue_2 ; If the player hits a wall
    (LocalVariables|SetVelocity%20Y 0.0) ; Set his Velocity Y to 0 so that he cant move in that direction
  )
  (return (* (Math|Vector2D|Normalize2D (Math|Vector2D|MakeVector2D (LocalVariables|GetVelocity%20X) (LocalVariables|GetVelocity%20Y))) (LocalVariables|GetVelocity%20Multiplier))))