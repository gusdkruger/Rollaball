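; BP_Shape is a destructible shape actor that breaks apart and awards score when the player touches it.
; On the first BoxCollision overlap with BP_Player, it sets a Hit flag and crumbles the root index cluster of its Geometry Collection.
; It then calls AddScore on GM_GameMode and destroys the collision box, so each shape scores only once.
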(event OnComponentBeginOverlap(BoxCollision)
  (params (OverlappedComponent :type Primitive%20Component%20Object%20Reference) (OtherActor :type Actor%20Object%20Reference) (OtherComp :type Primitive%20Component%20Object%20Reference) (OtherBodyIndex :type Integer) (bFromSweep :type Boolean) (SweepResult :type Hit%20Result%20Structure%20%28by%20ref%29))
  ;[0 0 0] Hit Player
  (if (not (Variables|Default|GetHit))
    (Utilities|Casting|CastToBP_Player OtherActor)
    (Variables|Default|SetHit true)
    (Class|GeometryCollectionComponent|CrumbleCluster (Variables|Default|GetGeometryCollection))
    (bind _asgm_game_mode (Utilities|Casting|CastToGM_GameMode (Game|GetGameMode)))
    (Default|AddScore _asgm_game_mode)
    (Components|DestroyComponent (Variables|Default|GetBoxCollision))))

(fn ConstructionScript)