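; Game mode for the start screen that shows the menu and can shatter the scene's shapes.
; On BeginPlay it creates the start screen widget, adds it to the viewport, and switches to UI-only input with the mouse cursor visible.
; A one-shot CrumbleAll event crumbles the geometry collection cluster of every BP_Shape actor and applies angular velocity to it.
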(event Custom|Crumble%20All
  ;[0 0 0] Crumble All
  (if (not (Variables|Default|GetCrumbed))
    (Variables|Default|SetCrumbed true)
    (bind _outactors (Actor|GetAllActorsOfClass "/Game/Actors/Shapes/BP_Shape.BP_Shape_C"))
    (for _array_element _outactors
      (Class|GeometryCollectionComponent|CrumbleCluster (Variables|/Game/Actors/Shapes/BP_Shape.BP_Shape_C|GetGeometryCollection _array_element))
      (Class|GeometryCollectionComponent|ApplyAngularVelocity (Variables|/Game/Actors/Shapes/BP_Shape.BP_Shape_C|GetGeometryCollection _array_element) 0 (Math|Vector|MakeVector 5e+02 0.0 0.0)))))

(event EventBeginPlay
  (bind _returnvalue (Game|GetPlayerController 0))
  ;[0 0 0] Begin Play
  (bind _returnvalue_2 (Game|ConstructObjectfromClass _returnvalue "/Game/UI/WBP_StartScreen.WBP_StartScreen_C"))
  (UserInterface|Viewport|AddtoViewport _returnvalue_2 0)
  (Input|SetInputModeUIOnly _returnvalue _returnvalue_2 "DoNotLock" false)
  (Variables|/Script/Engine.PlayerController|SetbShowMouseCursor _returnvalue true))

(fn ConstructionScript)