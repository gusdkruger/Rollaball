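; GM_GameMode is a game mode that tracks score against the number of BP_Shape actors in the level and ends the game when all are scored.
; On BeginPlay it sets game-only input, counts the shapes as MaxScore and shows the WBP_UI score widget.
; AddScore increments the score, refreshes the UI and, after a short delay once the maximum is reached, calls EndGame to show WBP_EndSreen with UI-only input and a cursor.
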(event Custom|End%20Game
  (bind _returnvalue (Game|GetPlayerController 0))
  ;[0 0 0] End Game
  (bind _returnvalue_2 (Game|ConstructObjectfromClass "/Game/UI/WBP_EndSreen.WBP_EndSreen_C"))
  (UserInterface|Viewport|AddtoViewport _returnvalue_2 0)
  (Input|SetInputModeUIOnly _returnvalue _returnvalue_2 "DoNotLock" true)
  (Variables|/Script/Engine.PlayerController|SetbShowMouseCursor _returnvalue true))

(event Custom|Add%20Score
  ;[0 0 0] Add Score
  (bind _result (Math|Integer|IncrementInt (Variables|Default|GetCurrent%20Score))
    (:%20%20
      (Default|UpdateScore (Variables|Default|GetUI) _result (Variables|Default|GetMax%20Score))
      (if (== (Variables|Default|GetCurrent%20Score) (Variables|Default|GetMax%20Score))
        (Utilities|FlowControl|Delay 1.0)
        (CallFunction|EndGame)))))

(event EventBeginPlay
  ;[0 0 0] Begin Play
  (Input|SetInputModeGameOnly (Game|GetPlayerController 0) false)
  (bind _outactors (Actor|GetAllActorsOfClass "/Game/Actors/Shapes/BP_Shape.BP_Shape_C"))
  (Variables|Default|SetMax%20Score (Utilities|Array|Length _outactors))
  (bind _returnvalue (Game|ConstructObjectfromClass "/Game/UI/WBP_UI.WBP_UI_C"))
  (bind _output_get (Variables|Default|SetUI _returnvalue))
  (UserInterface|Viewport|AddtoViewport _output_get 0)
  (Default|UpdateScore _returnvalue (Variables|Default|GetCurrent%20Score) (Variables|Default|GetMax%20Score)))

(fn ConstructionScript)